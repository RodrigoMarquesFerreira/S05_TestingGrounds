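; NPC_AI_BP is an NPC AI controller that runs the GuardBehaviour behavior tree using the PatrolData blackboard, both set up on BeginPlay.
; AI Perception updates feed the blackboard's Target key with any sensed actor not tagged Enemy.
; When sensing of such an actor fails, Target is set to an empty object; a ClearValue node is left unconnected.
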(event `self.ReceiveBeginPlay`
  ;[1 1 1] Set BlackBoard
  (bind _blackboardcomponent (`self.UseBlackboard` "/Game/Dynamic/NPCs/AI/PatrolData.PatrolData"))
  (set `self.BlackboardRef` _blackboardcomponent)
  (`self.RunBehaviorTree` "/Game/Dynamic/NPCs/AI/GuardBehaviour.GuardBehaviour"))

(event `self.AIPerception.OnTargetPerceptionUpdated`
  (params (Actor :type "Actor Object Reference") (Stimulus :type "AIStimulus Structure"))
  (bind _blackboardref (`self.BlackboardRef`))
  (if (`self.ActorHasTag` Actor "Enemy")
    _
    (elif (`.bSuccessfullySensed` (break `AIStimulus` Stimulus))
      (`BlackboardComponent.SetValueAsObject` _blackboardref "Target" Actor)
      (else
        (`BlackboardComponent.SetValueAsObject` _blackboardref "Target" null)))))

(fn `UserConstructionScript`)